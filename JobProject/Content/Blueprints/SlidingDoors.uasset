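; Sliding double door actor that opens for the player's E key or automatically for roaming and patrolling AI.
; A Doors timeline lerps two pivots between closed and open relative locations.
; Overlapping Box enables player input and plays the timeline for AI; any end overlap disables input and closes the doors, leaving DoorClosed unchanged.
; A second box toggles two open-door prompt widgets for the player.
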(event OnComponentBeginOverlap(Box)
  (params (OverlappedComponent :type Primitive%20Component%20Object%20Reference) (OtherActor :type Actor%20Object%20Reference) (OtherComp :type Primitive%20Component%20Object%20Reference) (OtherBodyIndex :type Integer) (bFromSweep :type Boolean) (SweepResult :type Hit%20Result%20Structure%20%28by%20ref%29))
  ;[1 0.2578 0.3175] Input
  (Utilities|FlowControl|Sequence
    (:then_0
      (Input|EnableInput (Game|GetPlayerController 0)))
    (:then_1
      (Utilities|Casting|CastToAi_roam_1 OtherActor)
      ;[0.8984 0 1] door open/close
      (bind _newtrack_0 (Timeline|doors Play)
        (:Update
          (Transformation|SetRelativeLocation (Variables|Default|Getpivot) (Math|Vector|Lerp(Vector) (Variables|Default|GetLeftDoorCurrent) (Variables|Default|GetLeftDoorNew) _newtrack_0) false false)
          (Transformation|SetRelativeLocation (Variables|Default|Getpivot1) (Math|Vector|Lerp(Vector) (Variables|Default|GetRightDoorCurrent) (Variables|Default|GetRightDoorNew) _newtrack_0) false false))))
    (:then_3
      (Utilities|Casting|CastToAiPotrol_1 OtherActor)
      (Timeline|doors Play))))

(event OnComponentEndOverlap(Box)
  (params (OverlappedComponent :type Primitive%20Component%20Object%20Reference) (OtherActor :type Actor%20Object%20Reference) (OtherComp :type Primitive%20Component%20Object%20Reference) (OtherBodyIndex :type Integer))
  ;[1 0.2578 0.3175] Input
  (Utilities|FlowControl|Sequence
    (:then_0
      (Input|DisableInput (Game|GetPlayerController 0)))
    (:then_1
      (Utilities|Casting|CastToAi_roam_1 OtherActor)
      ;[0.8984 0 1] door open/close
      (bind _newtrack_0 (Timeline|doors Reverse)
        (:Update
          (Transformation|SetRelativeLocation (Variables|Default|Getpivot) (Math|Vector|Lerp(Vector) (Variables|Default|GetLeftDoorCurrent) (Variables|Default|GetLeftDoorNew) _newtrack_0) false false)
          (Transformation|SetRelativeLocation (Variables|Default|Getpivot1) (Math|Vector|Lerp(Vector) (Variables|Default|GetRightDoorCurrent) (Variables|Default|GetRightDoorNew) _newtrack_0) false false))))
    (:then_2
      (Utilities|Casting|CastToAiPotrol_1 OtherActor)
      (Timeline|doors Reverse))
    (:then_3
      (Timeline|doors Reverse))))

(event OnComponentBeginOverlap(Box1)
  (params (OverlappedComponent :type Primitive%20Component%20Object%20Reference) (OtherActor :type Actor%20Object%20Reference) (OtherComp :type Primitive%20Component%20Object%20Reference) (OtherBodyIndex :type Integer) (bFromSweep :type Boolean) (SweepResult :type Hit%20Result%20Structure%20%28by%20ref%29))
  ;[1 1 1] text
  (Utilities|Casting|CastToPlayer OtherActor)
  (Rendering|SetVisibility (Variables|Default|GetWidget_opendoor) true false))

(event OnComponentEndOverlap(Box1)
  (params (OverlappedComponent :type Primitive%20Component%20Object%20Reference) (OtherActor :type Actor%20Object%20Reference) (OtherComp :type Primitive%20Component%20Object%20Reference) (OtherBodyIndex :type Integer))
  ;[1 1 1] text
  (Utilities|Casting|CastToPlayer OtherActor)
  (Rendering|SetVisibility (Variables|Default|GetWidget_opendoor) false false))

(event EventBeginPlay)

(event Collision|EventActorBeginOverlap
  (params (OtherActor :type Actor%20Object%20Reference)))

(event EventTick
  (params (DeltaSeconds :type Float%20%28single-precision%29)))

(event Input|KeyboardEvents|E
  (params (Key :type Key%20Structure :default "None"))
  ;[1 0.2578 0.3175] Input
  (:Pressed
    ;[0.8984 0 1] door open/close
    (if (Variables|Default|GetDoor_Closed?)
      (Variables|Default|SetDoor_Closed? false)
      (bind _newtrack_0 (Timeline|doors Play)
        (:Update
          (Transformation|SetRelativeLocation (Variables|Default|Getpivot) (Math|Vector|Lerp(Vector) (Variables|Default|GetLeftDoorCurrent) (Variables|Default|GetLeftDoorNew) _newtrack_0) false false)
          (Transformation|SetRelativeLocation (Variables|Default|Getpivot1) (Math|Vector|Lerp(Vector) (Variables|Default|GetRightDoorCurrent) (Variables|Default|GetRightDoorNew) _newtrack_0) false false)))
      (else
        (Variables|Default|SetDoor_Closed? true)
        (Timeline|doors Reverse)))))

(fn ConstructionScript)