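; Interactive cabinet with a drawer that slides open and closed when E is pressed.
; A bool toggles a timeline between play and reverse, scaling its track by LocationDistance to move the drawer along relative X.
; One collision volume enables input on any overlap and disables it on exit.
; A second volume shows the display widget only while the Player overlaps it.
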(event OnComponentBeginOverlap(OpenCabinetCollision)
  (params (OverlappedComponent :type Primitive%20Component%20Object%20Reference) (OtherActor :type Actor%20Object%20Reference) (OtherComp :type Primitive%20Component%20Object%20Reference) (OtherBodyIndex :type Integer) (bFromSweep :type Boolean) (SweepResult :type Hit%20Result%20Structure%20%28by%20ref%29))
  (Input|EnableInput (Game|GetPlayerController 0)))

(event OnComponentEndOverlap(OpenCabinetCollision)
  (params (OverlappedComponent :type Primitive%20Component%20Object%20Reference) (OtherActor :type Actor%20Object%20Reference) (OtherComp :type Primitive%20Component%20Object%20Reference) (OtherBodyIndex :type Integer))
  (Input|DisableInput (Game|GetPlayerController 0)))

(event OnComponentBeginOverlap(WidgetCollision)
  (params (OverlappedComponent :type Primitive%20Component%20Object%20Reference) (OtherActor :type Actor%20Object%20Reference) (OtherComp :type Primitive%20Component%20Object%20Reference) (OtherBodyIndex :type Integer) (bFromSweep :type Boolean) (SweepResult :type Hit%20Result%20Structure%20%28by%20ref%29))
  (Utilities|Casting|CastToPlayer OtherActor)
  (Rendering|SetVisibility (Variables|Default|GetDisplayWidget) true false))

(event OnComponentEndOverlap(WidgetCollision)
  (params (OverlappedComponent :type Primitive%20Component%20Object%20Reference) (OtherActor :type Actor%20Object%20Reference) (OtherComp :type Primitive%20Component%20Object%20Reference) (OtherBodyIndex :type Integer))
  (Utilities|Casting|CastToPlayer OtherActor)
  (Rendering|SetVisibility (Variables|Default|GetDisplayWidget) false false))

(event Input|KeyboardEvents|E
  (params (Key :type Key%20Structure))
  (:Pressed
    (if (Variables|Default|GetOpenCabinet?)
      (Variables|Default|SetOpenCabinet? false)
      (bind _newtrack_0 (Timeline|Timeline_0 Play)
        (:Update
          (Transformation|SetRelativeLocation (Variables|Default|GetDrawer) (Math|Vector|MakeVector (* _newtrack_0 (Variables|Default|Getlocation%20_distance)) 0.0 29.0) false false)))
      (else
        (Variables|Default|SetOpenCabinet? true)
        (Timeline|Timeline_0 Reverse)))))

(fn ConstructionScript)